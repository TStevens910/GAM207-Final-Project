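; AI controller that runs the AI_BT behavior tree on BeginPlay and reacts to perception updates.
; When a perceived actor is an AICharacter_BP or Bp_Character, it stores it as TargetEnemy and writes the stimulus location to the Destination blackboard key.
; The branch is fixed to true, so the target-clearing path never runs.
; The node that would write TargetEnemy to EnemyActor is disconnected.
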(event OnTargetPerceptionUpdated(AIPerception)
  (params (Actor :type Actor%20Object%20Reference) (Stimulus :type AI%20Stimulus%20Structure))
  (bind _returnvalue (AI|GetBlackboard 0))
  ;[0.15 0.15 0.15 0.5] AI Perception
  (Utilities|Casting|CastToAICharacter_BP Actor
    (:then
      _)
    (:CastFailed
      (Utilities|Casting|CastToBp_Character Actor)))
  (if true
    (bind _output_get (Variables|Default|SetTargetEnemy Actor))
    (Utilities|IsValid _returnvalue
      (:Is%20Valid
        (AI|Components|Blackboard|SetValueasVector (AI|GetBlackboard 0) (Utilities|Name|MakeLiteralName "Destination") (.StimulusLocation (Utilities|Struct|BreakAIStimulus Stimulus)))))
    (else
      (Variables|Default|SetTargetEnemy 0)
      (AI|Components|Blackboard|SetValueasObject _returnvalue (Utilities|Name|MakeLiteralName "EnemyActor") 0))))

(event EventBeginPlay
  ;[0.15 0.15 0.15 0.5] BeginPlay
  (AI|RunBehaviorTree "/Game/AI/AI_BT.AI_BT"))

(fn ConstructionScript)